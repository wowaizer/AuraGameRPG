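; Gameplay Ability that makes an enemy play its hit reaction.
; On activation it applies GE_HitReact to the owner, storing the handle, then gets the montage from the avatar's CombatInterface and calls HitReaction(true).
; The montage plays at double rate; completion, interruption or cancellation all remove the effect, end the ability and call HitReaction(false).
; A failed interface cast stops execution without removing the effect or ending the ability.
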(event Ability|EventActivateAbility
  (Variables|Default|SetIs%20Hit true)
  (bind _returnvalue (Ability|ApplyGameplayEffectToOwner "/Game/BluePrints/AbilitySystem/Enemies/Effects/GE_HitReact.GE_HitReact_C"))
  (Variables|Default|SetActiveGE_HitReact _returnvalue)
  (bind _ascombat_interface (Utilities|Casting|CastToCombatInterface (Ability|GetAvatarActorfromActorInfo)))
  (bind _returnvalue_2 (Class|CombatInterface|GetHitReactMontage _ascombat_interface))
  (Class|CombatInterface|HitReaction _ascombat_interface (Variables|Default|GetIs%20Hit))
  (|PlayMontageandWaitProxy "None" _returnvalue_2 2.0 "None" true 1.0 0.0
    (:OnCompleted
      _)
    (:OnInterrupted
      _)
    (:OnCancelled
      _))
  (Ability|RemoveGameplayEffectFromOwnerWithHandle (Variables|Default|GetActiveGE_HitReact))
  (Ability|EndAbility)
  (bind _output_get (Variables|Default|SetIs%20Hit false))
  (Class|CombatInterface|HitReaction _ascombat_interface _output_get))

(event Ability|EventOnEndAbility
  (params (bWasCancelled :type Boolean)))